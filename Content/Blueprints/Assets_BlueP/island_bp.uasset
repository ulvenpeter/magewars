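; Island actor that wanders endlessly between randomly chosen waypoints in the level.
; On BeginPlay it collects TargetPoints tagged "Island_1" and picks one at random as the current target.
; Each Tick it advances along its forward vector by a fixed, frame-rate-dependent step while smoothly turning toward the target with RInterpTo.
; When within one unit of the target it picks another at random, possibly the same one.
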(event EventBeginPlay
  (bind _targetarray (Variables|Default|GetTargetArray))
  (bind _outactors (Actor|GetAllActorsOfClass "/Script/Engine.TargetPoint"))
  (for _array_element _outactors
    (if (Actor|ActorHasTag _array_element "Island_1")
      (Utilities|Array|Add (Variables|Default|GetTargetArray) _array_element)))
  (Variables|Default|SetCurrentTarget (Utilities|Array|Get(acopy) _targetarray (Math|Random|RandomIntegerinRange 0 (Utilities|Array|LastIndex _targetarray)))))

(event EventTick
  (params (DeltaSeconds :type Float%20%28single-precision%29))
  (bind _targetarray (Variables|Default|GetTargetArray))
  (Transformation|SetActorLocationAndRotation (+ (Transformation|GetActorLocation) (+ (Transformation|GetActorForwardVector) 0.0)) (Math|Interpolation|RInterpTo (Transformation|GetActorRotation) (Math|Rotator|FindLookatRotation (Transformation|GetActorLocation) (Transformation|GetActorLocation (Variables|Default|GetCurrentTarget))) (Utilities|Time|GetWorldDeltaSeconds) 1.0))
  (if (< (Transformation|GetDistanceTo (Variables|Default|GetCurrentTarget)) 1.0)
    (Variables|Default|SetCurrentTarget (Utilities|Array|Get(acopy) _targetarray (Math|Random|RandomIntegerinRange 0 (Utilities|Array|LastIndex _targetarray))))))

(fn ConstructionScript)