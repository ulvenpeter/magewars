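; BlueTower_BP is a blue crystal tower actor with continuously spinning rings and crystals.
; Each Tick applies incremental rotations to three circle meshes, the core circles, and the mother and baby crystal meshes, using separate speed variables on set axes.
; The core tumbles on all three axes while crystals spin on yaw.
; Rotation steps are not scaled by delta time, so spin speed depends on frame rate.
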(event EventTick
  (params (DeltaSeconds :type Float%20%28single-precision%29))
  (bind _corespeed (Variables|Default|GetCoreSpeed))
  (Transformation|AddLocalRotation (Variables|Default|Getcircles_tower_circle1) (Math|Rotator|MakeRotator (Variables|Default|GetCircle01Speed) 0.0 0.0) false false)
  (Transformation|AddRelativeRotation (Variables|Default|Getcircles_tower_circle2) (Math|Rotator|MakeRotator (Variables|Default|GetCircle02Speed) 0.0 0.0) false false)
  (Transformation|AddLocalRotation (Variables|Default|Getcircles_tower_circle3) (Math|Rotator|MakeRotator 0.0 (Variables|Default|GetCircle03Speed) 0.0) false false)
  (Transformation|AddLocalRotation (Variables|Default|Getcircles_tower_corecircles) (Math|Rotator|MakeRotator _corespeed _corespeed _corespeed) false false)
  (Transformation|AddLocalRotation (Variables|Default|GetTowerBlueLowPoly__1__mothercrystals) (Math|Rotator|MakeRotator 0.0 0.0 (Variables|Default|GetBigCrystalSpeed)) false false)
  (Transformation|AddLocalRotation (Variables|Default|GetTowerBlueLowPoly__1__babycrystals) (Math|Rotator|MakeRotator 0.0 0.0 (Variables|Default|GetSmallCrystalSpeed)) false false))

(fn ConstructionScript)